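; Door trigger actor (Puerta) that moves the game to another level when any actor overlaps it.
; On overlap it stores the target position and rotation in the Global_vars game instance and sets its Reubicar flag, presumably for repositioning after loading.
; It then adds a Fade widget to the viewport, opens the level named by NombreNivel after a short delay, and prints a debug message.
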(event `self.ReceiveActorBeginOverlap`
  (params (OtherActor :type "Actor Object Reference"))
  (`|ExecutionSequence`
    (:`then_0`
      (bind _asglobal_vars (cast `/Game/Blueprints/Global_vars` (`GameplayStatics.GetGameInstance`)))
      (set `/Game/Blueprints/Global_vars.Reubicar` true _asglobal_vars)
      (set `/Game/Blueprints/Global_vars.Reubicar_pos` (`self.Nueva_posicion`) _asglobal_vars)
      (set `/Game/Blueprints/Global_vars.Reubicar_rot` (`self.Nueva_rot`) _asglobal_vars))
    (:`then_1`
      (bind _returnvalue (`|CreateWidget` "/Game/Widgets_recorrido/Recorrido/Fade.Fade_C"))
      (`UserWidget.AddToViewport` _returnvalue 0))
    (:`then_2`
      (`KismetSystemLibrary.Delay` 1.0)
      (`GameplayStatics.OpenLevel` (`self.Nombre_nivel`)))
    (:`then_3`
      (`KismetSystemLibrary.PrintString` "Trigger" true true (struct :`R` 1.0 :`G` 0.045833 :`B` 0.867254 :`A` 1.0)))))

(fn `UserConstructionScript`)