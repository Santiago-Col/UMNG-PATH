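; Player character for a location-based mobile game that maps the real-world Calle100 or Cajica site, chosen by PlayInCalle100, into the level.
; When flagged as on-site, a one-second timer converts GPS offsets from the site origin into centimetres and relocates the character, while device rotation rate drives the view on Tick.
; When off-site, movement axes walk the character relative to control yaw.
; Turn and look-up axes work in both modes.
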(event `self.ReceiveTick`
  (params (DeltaSeconds :type "Float (single-precision)"))
  (bind (_tilt _rotationrate) (`PlayerController.GetInputMotionState` (`GameplayStatics.GetPlayerController` 0)))
  (if (`self.PlayInCalle100`)
    (if (`self.IsInCalle100`)
      (`|ExecutionSequence` :!label _label
        (:`then_0`
          (`self.AddControllerYawInput` (* (.y _rotationrate) -40.0 (`GameplayStatics.GetWorldDeltaSeconds`))))
        (:`then_1`
          (`self.AddControllerPitchInput` (* (.x _rotationrate) -40.0 (`GameplayStatics.GetWorldDeltaSeconds`))))))
    (elif (`self.IsInCajica`)
      (goto _label))))

(event `self.ReceiveBeginPlay`
  (bind _returnvalue (`LocationServices.InitLocationServices` "LA_TenMeters"))
  (bind _output_get (set `self.Init location services` _returnvalue))
  (if _output_get
    (`KismetSystemLibrary.K2_SetTimerDelegate` (delegate `MoveActor`) 1.0 true)))

(event `MoveActor`
  (if (`self.PlayInCalle100`)
    (if (`self.IsInCalle100`)
      (`LocationServices.StartLocationServices`)
      (bind _returnvalue (`LocationServices.GetLastKnownLocation`))
      (bind _output_get (set `self.CoorD` (`KismetMathLibrary.MakeVector` (- (`.Latitude` (break `LocationServicesData` _returnvalue)) (`self.LatCalle100`)) (- (`.Longitude` (break `LocationServicesData` _returnvalue)) (`self.LongCalle100`)))))
      (`self.K2_SetActorLocation` (`GameplayStatics.GetPlayerCharacter` 0) (+ (* (* _output_get 111.120003) 100000) (0.0 0.0 112.0)) false false))
    (elif (`self.IsInCajica`)
      (`LocationServices.StartLocationServices`)
      (bind _returnvalue_2 (`LocationServices.GetLastKnownLocation`))
      (bind _output_get_2 (set `self.CoorD` (`KismetMathLibrary.MakeVector` (- (`.Latitude` (break `LocationServicesData` _returnvalue_2)) (`self.LatCajica`)) (- (`.Longitude` (break `LocationServicesData` _returnvalue_2)) (`self.LongCajica`)))))
      (`self.K2_SetActorLocation` (`GameplayStatics.GetPlayerCharacter` 0) (+ (* (* _output_get_2 111.120003) 100000) (0.0 0.0 112.0)) false false))))

(event `InputAxis|MoveForward`
  (params (AxisValue :type "Float (single-precision)"))
  (if (`self.PlayInCalle100`)
    (if (not (`self.IsInCalle100`))
      (`self.AddMovementInput` (`KismetMathLibrary.GetForwardVector` (`KismetMathLibrary.MakeRotator` 0.0 0.0 (.yaw (`self.GetControlRotation`)))) AxisValue :!label _label_2))
    (elif (not (`self.IsInCajica`))
      (goto _label_2))))

(event `InputAxis|TurnRate`
  (params (AxisValue :type "Float (single-precision)"))
  (if (`self.PlayInCalle100`)
    (if (`self.IsInCalle100`)
      _
      (else
        _))
    (elif (`self.IsInCajica`)
      _
      (else
        _)))
  (`self.AddControllerYawInput` (* AxisValue 45.0 (`GameplayStatics.GetWorldDeltaSeconds`))))

(event `InputAxis|LookUpRate`
  (params (AxisValue :type "Float (single-precision)"))
  (if (`self.PlayInCalle100`)
    (if (`self.IsInCalle100`)
      _
      (else
        _))
    (elif (`self.IsInCajica`)
      _
      (else
        _)))
  (`self.AddControllerPitchInput` (* AxisValue 45.0 (`GameplayStatics.GetWorldDeltaSeconds`))))

(event `InputAxis|MoveRight`
  (params (AxisValue :type "Float (single-precision)"))
  (if (`self.PlayInCalle100`)
    (if (not (`self.IsInCalle100`))
      (`self.AddMovementInput` (`KismetMathLibrary.GetRightVector` (`KismetMathLibrary.MakeRotator` 0.0 0.0 (.yaw (`self.GetControlRotation`)))) AxisValue :!label _label_3))
    (elif (not (`self.IsInCajica`))
      (goto _label_3))))

(fn `UserConstructionScript`)